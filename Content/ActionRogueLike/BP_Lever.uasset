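; BP_Lever is an interactable lever that triggers a selected actor when switched on.
; Each Interact toggles its ON state and updates the lever mesh's pitch from a stored Rotation value.
; When on, it directly explodes a selected BP_ExplosiveBarrel, or forwards an Interact message with the instigating pawn to any other selected actor.
; Switching off only moves the lever.
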(event `SGamePlayInterface.Interact`
  (params (InstigationPawn :type "Pawn Object Reference"))
  (bind _selectedactor (`self.SelectedActor`))
  (bind _output_get (set `self.ON` (not (`self.ON`))))
  (bind _result (`/Engine/EditorBlueprintResources/StandardMacros.NegateFloat` (`self.Rotation`))
    (:`  `
      (bind _output_get_2 (set `self.Rotation` _result))
      (`SceneComponent.K2_SetRelativeRotation` (`self.LeverMesh`) (`KismetMathLibrary.MakeRotator` 0.0 _output_get_2) false false)
      (if _output_get
        (bind _asbp_explosive_barrel (cast `/Game/ActionRogueLike/BP_ExplosiveBarrel` _selectedactor)
          (:`then`
            (`/Game/ActionRogueLike/BP_ExplosiveBarrel.Explode` _asbp_explosive_barrel))
          (:`CastFailed`
            (message `SGamePlayInterface.Interact` _selectedactor InstigationPawn)))))))

(fn `UserConstructionScript`)